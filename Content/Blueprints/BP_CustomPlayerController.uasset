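; Player controller for a first-person tower-defense game, handling wave triggering, shop toggling, defense placement, upgrades and money gain.
; The mode key traces from the camera to activate a wave button, otherwise flip-flops between shop and HUD widgets.
; Placement spawns one of two towers or a frozen zone, ignoring Visibility while following the cursor until mouse release.
; Per-type upgrade levels apply to every placed instance through tracked arrays.
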(event `EnhancedInput|/Game/Input/Actions/IA_ChangeMode`
  (params (ActionValue :type Boolean) (ElapsedSeconds :type "Float (double-precision)") (TriggeredSeconds :type "Float (double-precision)") (InputAction :type "InputAction Object Reference" :default "/Game/Input/Actions/IA_ChangeMode.IA_ChangeMode"))
  (bind _firstpersoncamera (`/Game/Blueprints/BP_FirstPersonCharacter.FirstPersonCamera` (`self.PlayerRef`)))
  (bind _returnvalue (`SceneComponent.K2_GetComponentLocation` _firstpersoncamera))
  (:`Started`
    (bind _outhit (`KismetSystemLibrary.LineTraceSingle` :`Start` _returnvalue :`End` (+ _returnvalue (* (`SceneComponent.GetForwardVector` _firstpersoncamera) 5000.0)) :`TraceChannel` "TraceTypeQuery1" :`DrawDebugType` "ForDuration"))
    (bind _asbp_button_wave (cast `/Game/Blueprints/BP_ButtonWave` (`.HitActor` (`GameplayStatics.BreakHitResult` _outhit)))
      (:`then`
        (`/Game/Blueprints/Spawner/BP_SpanwerMaster.CheckEnnemyOnMap` (`self.MasterRef`))
        (`/Game/Blueprints/BP_ButtonWave.Active` _asbp_button_wave))
      (:`CastFailed`
        (`/Engine/EditorBlueprintResources/StandardMacros.FlipFlop`
          (:`A`
            (bind _returnvalue_2 (`|CreateWidget` "/Game/UI/WG_Shop.WG_Shop_C" null self))
            (bind _output_get (set `self.InterfaceRef` _returnvalue_2))
            (`UserWidget.AddToViewport` _output_get 0)
            (bind _output_get_2 (set `self.bShowMouseCursor` true))
            (bind _output_get_3 (set `self.b_OnInventory` _output_get_2))
            (`/Game/Blueprints/BP_FirstPersonCharacter.Oninventory` (`self.PlayerRef`) (not _output_get_3)))
          (:`B`
            (`WidgetLayoutLibrary.RemoveAllWidgets`)
            (bind _output_get_4 (set `self.bShowMouseCursor` false))
            (bind _output_get_5 (set `self.b_OnInventory` _output_get_4))
            (`/Game/Blueprints/BP_FirstPersonCharacter.Oninventory` (`self.PlayerRef`) (not _output_get_5))
            (bind _returnvalue_3 (`|CreateWidget` "/Game/UI/WG_Interface.WG_Interface_C"))
            (`UserWidget.AddToViewport` _returnvalue_3 0)))))))

(event `self.ReceiveTick`
  (params (DeltaSeconds :type "Float (single-precision)"))
  (bind _hitresult (`self.GetHitResultUnderCursorByChannel` "TraceTypeQuery1"))
  (if (`self.b_Placing`)
    (if (`GameplayStatics.BreakHitResult` _hitresult)
      (switch `int` (`self.Selection`)
        (:`Default`
          (`self.K2_SetActorLocation` (`self.CurrentTower`) (`.ImpactPoint` (`GameplayStatics.BreakHitResult` _hitresult)) false false :!label _label))
        (:`0`
          (goto _label))
        (:`1`
          (`self.K2_SetActorLocation` (`self.CurrentFrozenZone`) (`.ImpactPoint` (`GameplayStatics.BreakHitResult` _hitresult)) false false))
        (:`2`
          (`self.K2_SetActorLocation` (`self.CurrentTower02`) (`.ImpactPoint` (`GameplayStatics.BreakHitResult` _hitresult)) false false))))))

(event `Upgrade`
  (params (WhatUpgrade :type Integer))
  (switch `int` WhatUpgrade
    (:`0`
      (bind _output_get (set `self.UpgradeLVLTurret1` (+ (`self.UpgradeLVLTurret1`) 1)))
      (`self.UpgradeTower` _output_get))
    (:`1`
      (bind _output_get_2 (set `self.LVLOfFrozenZone` (+ (`self.LVLOfFrozenZone`) 1)))
      (`self.UpgradeFrozenZone` _output_get_2))
    (:`2`
      (bind _output_get_3 (set `self.LVLOfTower02` (+ (`self.LVLOfTower02`) 1)))
      (`self.UpgradeTower2` _output_get_3))))

(event `Key|LeftMouseButton`
  (params (Key :type "Key Structure"))
  (:`Released`
    (if (`self.b_OnInventory`)
      (`self.CurrentTower`
        (:`then`
          (set `self.b_Placing` false)
          (`PrimitiveComponent.SetCollisionResponseToChannel` (`/Game/Blueprints/Defence/BP_Tower01.StaticMesh` (`self.CurrentTower`)) "ECC_Visibility" "ECR_Block")
          (`/Game/Blueprints/Defence/BP_Tower01.ActiveTurret` (`self.CurrentTower`)))
        (:`else`
          (`self.CurrentFrozenZone`
            (:`then`
              (set `self.b_Placing` false)
              (`PrimitiveComponent.SetCollisionResponseToChannel` (`/Game/Blueprints/Defence/BP_FreezenZone.FrozenZone` (`self.CurrentFrozenZone`)) "ECC_Visibility" "ECR_Block"))
            (:`else`
              (bind _currenttower02 (`self.CurrentTower02`)
                (:`then`
                  (set `self.b_Placing` false)
                  (`PrimitiveComponent.SetCollisionResponseToChannel` (`/Game/Blueprints/Defence/BP_Tower02.StaticMesh` _currenttower02) "ECC_Visibility" "ECR_Block")
                  (`/Game/Blueprints/Defence/BP_Tower02.ActiveTurret` (`self.CurrentTower02`)))
                (:`else`)))))))))

(event `GainMoney`
  (params (Gain :type "Float (double-precision)"))
  (set `self.Money` (+ (`self.Money`) Gain)))

(event `self.ReceiveBeginPlay`
  (bind _returnvalue (`GameplayStatics.GetActorOfClass` "/Game/Blueprints/BP_FirstPersonCharacter.BP_FirstPersonCharacter_C"))
  (set `self.PlayerRef` _returnvalue)
  (bind _returnvalue_2 (`GameplayStatics.GetActorOfClass` "/Game/Blueprints/Spawner/BP_SpanwerMaster.BP_SpanwerMaster_C"))
  (set `self.MasterRef` _returnvalue_2)
  (bind _returnvalue_3 (`|CreateWidget` "/Game/UI/WG_Tuto.WG_Tuto_C"))
  (`UserWidget.AddToViewport` _returnvalue_3 0)
  (set `self.bShowMouseCursor` true))

(event `StartSession`
  (`WidgetLayoutLibrary.RemoveAllWidgets`)
  (set `self.bShowMouseCursor` false)
  (bind _returnvalue (`|CreateWidget` "/Game/UI/WG_Interface.WG_Interface_C"))
  (`UserWidget.AddToViewport` _returnvalue 0))

(event `EventPlacingMode`
  (params (Selection :type Integer))
  (bind _output_get (set `self.Selection` Selection))
  (if (not (`self.b_Placing`))
    (set `self.b_Placing` true)
    (switch `int` _output_get
      (:`Default`
        (bind _returnvalue (`|SpawnActorFromClass` "/Game/Blueprints/Defence/BP_Tower01.BP_Tower01_C" (`KismetMathLibrary.MakeTransform` (0.0 0.0 0.0)) "Undefined" "OverrideRootScale" null null :!label _label_2))
        (bind _output_get_2 (set `self.CurrentTower` _returnvalue))
        (`PrimitiveComponent.SetCollisionResponseToChannel` (`/Game/Blueprints/Defence/BP_Tower01.StaticMesh` _output_get_2) "ECC_Visibility" "ECR_Ignore")
        (`KismetArrayLibrary.Array_Add` (`self.ArrayOfTower01`) (`self.CurrentTower`))
        (`self.UpgradeTower` (`self.UpgradeLVLTurret1`)))
      (:`0`
        (goto _label_2))
      (:`1`
        (bind _returnvalue_2 (`|SpawnActorFromClass` "/Game/Blueprints/Defence/BP_FreezenZone.BP_FreezenZone_C" (`KismetMathLibrary.MakeTransform` (0.0 0.0 0.0)) "Undefined" "OverrideRootScale" null null))
        (bind _output_get_3 (set `self.CurrentFrozenZone` _returnvalue_2))
        (`PrimitiveComponent.SetCollisionResponseToChannel` (`/Game/Blueprints/Defence/BP_FreezenZone.FrozenZone` _output_get_3) "ECC_Visibility" "ECR_Ignore")
        (`KismetArrayLibrary.Array_Add` (`self.ArrayOfFrozenZone`) (`self.CurrentFrozenZone`))
        (`self.UpgradeFrozenZone` (`self.LVLOfFrozenZone`)))
      (:`2`
        (bind _returnvalue_3 (`|SpawnActorFromClass` "/Game/Blueprints/Defence/BP_Tower02.BP_Tower02_C" (`KismetMathLibrary.MakeTransform` (0.0 0.0 0.0)) "Undefined" "OverrideRootScale" null null))
        (bind _output_get_4 (set `self.CurrentTower02` _returnvalue_3))
        (`PrimitiveComponent.SetCollisionResponseToChannel` (`/Game/Blueprints/Defence/BP_Tower02.StaticMesh` _output_get_4) "ECC_Visibility" "ECR_Ignore")
        (`KismetArrayLibrary.Array_Add` (`self.ArrayOfTower02`) (`self.CurrentTower02`))
        (`self.UpgradeTower2` (`self.LVLOfTower02`))))))

(fn `UpgradeFrozenZone`
  (params (Selection :type Integer))
  (locals (UpgradeAS :type "Float (double-precision)" :default 2.0))
  (switch `int` Selection
    (:`1`
      (set `local.UpgradeAS` 70.0))
    (:`2`
      (set `local.UpgradeAS` 100.0))
    (:`3`
      (set `local.UpgradeAS` 120.0)))
  (for _array_element (`self.ArrayOfFrozenZone`)
    (bind _output_get (set `/Game/Blueprints/Defence/BP_FreezenZone.Slow%` (`local.UpgradeAS`) _array_element))
    (`KismetSystemLibrary.PrintString` (`KismetStringLibrary.Conv_DoubleToString` _output_get))))

(fn `UpgradeTower`
  (params (LevelOfTurret :type Integer))
  (locals (UpgradeAS :type "Float (double-precision)"))
  (switch `int` LevelOfTurret
    (:`1`
      (set `local.UpgradeAS` 2.0))
    (:`2`
      (set `local.UpgradeAS` 3.0))
    (:`3`
      (set `local.UpgradeAS` 4.0)))
  (for _array_element (`self.ArrayOfTower01`)
    (bind _output_get (set `/Game/Blueprints/Defence/BP_Tower01.AttackSpeed` (`local.UpgradeAS`) _array_element))
    (`KismetSystemLibrary.PrintString` (`KismetStringLibrary.Conv_DoubleToString` _output_get))))

(fn `UpgradeTower2`
  (params (LVL :type Integer))
  (locals (UpgradeAS :type "Float (double-precision)" :default 2.0))
  (switch `int` LVL
    (:`Default`
      (for _array_element (`self.ArrayOfTower02`) :!label _label
        (if (not (`/Game/Blueprints/Defence/BP_Tower02.b_CanShoot2` _array_element))
          (`/Game/Blueprints/Defence/BP_Tower02.Upgrade` _array_element))))
    (:`0`
      (goto _label))
    (:`1`
      (for _array_element_2 (`self.ArrayOfTower02`)
        (`/Game/Blueprints/Defence/BP_Tower02.Upgrade` _array_element_2)))))

(fn `UserConstructionScript`)