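; BP_Ennemy03 is an enemy that walks along a spline path with a looping walk animation, apparently for a tower-defense mode.
; A Timeline, started shortly after BeginPlay at a play rate of 1/Speed, drives location and tangent-based rotation by distance along the spline.
; ResetSpeed restores the initial speed after a delay.
; Lethal damage prints placeholder FX, awards money, notifies the spawner master and destroys the actor.
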(event `ResetSpeed`
  (params (Duration :type "Float (single-precision)"))
  (`KismetSystemLibrary.Delay` Duration)
  (bind _output_get (set `self.Speed` (`self.InitialSpeed`)))
  (`TimelineComponent.SetPlayRate` (`self.Timeline`) (/ 1.0 _output_get)))

(event `TakeDamage`
  (params (B :type "Float (double-precision)"))
  (bind _output_get (set `self.LifePoint` (- (`self.LifePoint`) B)))
  (if (<= _output_get 0.0)
    (`KismetSystemLibrary.PrintString` "FX") ; A changer par des FX
    (`/Game/Blueprints/BP_CustomPlayerController.GainMoney` (`self.PlayerRef`) (`self.Price`))
    (`/Game/Blueprints/Spawner/BP_SpanwerMaster.CheckEnnemyOnMap` (`self.SpawnerMasterRef`))
    (`self.K2_DestroyActor`)))

(event `self.ReceiveBeginPlay`
  (bind _spline (`/Game/Blueprints/Spline_Mouvement/BP_Spline.Spline` (`self.Spline`)))
  (`|ExecutionSequence`
    (:`then_0`
      (bind _returnvalue (`GameplayStatics.GetActorOfClass` "/Game/Blueprints/Spawner/BP_SpanwerMaster.BP_SpanwerMaster_C"))
      (set `self.SpawnerMasterRef` _returnvalue))
    (:`then_1`
      (bind _returnvalue_2 (`GameplayStatics.GetActorOfClass` "/Game/Blueprints/BP_CustomPlayerController.BP_CustomPlayerController_C"))
      (set `self.PlayerRef` _returnvalue_2))
    (:`then_2`
      (`SkeletalMeshComponent.PlayAnimation` (`self.Mesh`) "/Game/Anims/Elf_WalkWalking.Elf_WalkWalking" true))
    (:`then_3`
      (`KismetSystemLibrary.Delay` 0.5)
      (`TimelineComponent.SetPlayRate` (`self.Timeline`) (/ 1.0 (`self.Speed`)))
      (bind (_direction _newtrack_0) (`Timeline|Timeline` :!via `PlayFromStart`)
        (:`Update`
          (bind _returnvalue_3 (`KismetMathLibrary.Lerp` 0.0 (`SplineComponent.GetDistanceAlongSplineAtSplinePoint` _spline (- (`SplineComponent.GetNumberOfSplinePoints` _spline) 1)) _newtrack_0))
          (`self.K2_SetActorLocation` (`SplineComponent.GetLocationAtDistanceAlongSpline` _spline _returnvalue_3 "World"))
          (`self.K2_SetActorRotation` (`KismetMathLibrary.Conv_VectorToRotator` (`SplineComponent.GetTangentAtDistanceAlongSpline` _spline _returnvalue_3 "World"))))))))

(fn `UserConstructionScript`)