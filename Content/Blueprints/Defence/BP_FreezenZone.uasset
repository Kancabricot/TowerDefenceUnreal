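; Defence freeze zone Blueprint that temporarily slows enemies entering its trigger volume.
; On overlap, ModifySpeed casts the actor to one of three enemy classes and adds the Slow amount to its Speed.
; Speed acts inversely: the enemy's Timeline play rate becomes 1/Speed, so a larger value means slower movement.
; Each branch then calls the enemy's ResetSpeed with DurationOfSlow.
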(event `self.TriggerZone.OnComponentBeginOverlap`
  (params (OverlappedComponent :type "PrimitiveComponent Object Reference") (OtherActor :type "Actor Object Reference") (OtherComp :type "PrimitiveComponent Object Reference") (OtherBodyIndex :type Integer) (bFromSweep :type Boolean) (SweepResult :type "HitResult Structure (by ref)"))
  (bind _result (`/Engine/EditorBlueprintResources/StandardMacros.NegateFloat` (`self.Slow%`))
    (:`  `
      (`self.ModifySpeed` OtherActor _result))))

(fn `ModifySpeed`
  (params (Target :type "Actor Object Reference") (`Slow%` :type "Float (double-precision)"))
  (locals (DurationOfSlow :type "Float (single-precision)" :default 2.0))
  (bind _durationofslow (`local.DurationOfSlow`))
  (bind _asbp_ennemy_01 (cast `/Game/Blueprints/Ennemy/BP_Ennemy01` Target)
    (:`then`
      (bind _output_get (set `/Game/Blueprints/Ennemy/BP_Ennemy01.Speed` (+ (`/Game/Blueprints/Ennemy/BP_Ennemy01.Speed` _asbp_ennemy_01) `Slow%`) _asbp_ennemy_01))
      (`TimelineComponent.SetPlayRate` (`/Game/Blueprints/Ennemy/BP_Ennemy01.Timeline` _asbp_ennemy_01) (/ 1.0 _output_get))
      (`/Game/Blueprints/Ennemy/BP_Ennemy01.ResetSpeed` _asbp_ennemy_01 _durationofslow))
    (:`CastFailed`
      (bind _asbp_ennemy_02 (cast `/Game/Blueprints/Ennemy/BP_Ennemy02` Target)
        (:`then`
          (bind _output_get_2 (set `/Game/Blueprints/Ennemy/BP_Ennemy02.Speed` (+ (`/Game/Blueprints/Ennemy/BP_Ennemy02.Speed` _asbp_ennemy_02) `Slow%`) _asbp_ennemy_02))
          (`TimelineComponent.SetPlayRate` (`/Game/Blueprints/Ennemy/BP_Ennemy02.Timeline` _asbp_ennemy_02) (/ 1.0 _output_get_2))
          (`/Game/Blueprints/Ennemy/BP_Ennemy02.ResetSpeed` _asbp_ennemy_02 _durationofslow))
        (:`CastFailed`
          (bind _asbp_ennemy_03 (cast `/Game/Blueprints/Ennemy/BP_Ennemy03` Target))
          (bind _output_get_3 (set `/Game/Blueprints/Ennemy/BP_Ennemy03.Speed` (+ (`/Game/Blueprints/Ennemy/BP_Ennemy03.Speed` _asbp_ennemy_03) `Slow%`) _asbp_ennemy_03))
          (`TimelineComponent.SetPlayRate` (`/Game/Blueprints/Ennemy/BP_Ennemy03.Timeline` _asbp_ennemy_03) (/ 1.0 _output_get_3))
          (`/Game/Blueprints/Ennemy/BP_Ennemy03.ResetSpeed` _asbp_ennemy_03 (`local.DurationOfSlow`)))))))

(fn `UserConstructionScript`)