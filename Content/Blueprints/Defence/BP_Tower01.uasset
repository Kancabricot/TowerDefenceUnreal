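; Defence tower that, once ActiveTurret enables it and removes its pre-reveal hitbox, damages enemies inside its trigger box.
; Overlaps maintain a target array of the three BP_Ennemy types, and each new overlap calls Shoot.
; Shoot hits the first target with a smoke burst and repeats after AttackSpeed, stopping when the attack fails.
; A LookTarget helper rotates the mesh but is never called here.
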(event `Shoot`
  (if (`self.b_IsActive`)
    (if (>= (`KismetArrayLibrary.Array_Length` (`self.ArrayOfTarget`)) 0)
      (bind _b_continue (`self.Attack` 0))
      (if _b_continue
        (`KismetSystemLibrary.Delay` (`self.AttackSpeed`))
        (`self.Shoot`)))))

(event `ActiveTurret`
  (set `self.b_IsActive` true)
  (bind _prerevealhitbox (`self.PreRevealHitbox`)
    (:`then`
      (`ActorComponent.K2_DestroyComponent` _prerevealhitbox))
    (:`else`)))

(event `self.TriggerBox.OnComponentBeginOverlap`
  (params (OverlappedComponent :type "PrimitiveComponent Object Reference") (OtherActor :type "Actor Object Reference") (OtherComp :type "PrimitiveComponent Object Reference") (OtherBodyIndex :type Integer) (bFromSweep :type Boolean) (SweepResult :type "HitResult Structure (by ref)"))
  (`self.AddInArray` OtherActor)
  (`self.Shoot`))

(event `self.TriggerBox.OnComponentEndOverlap`
  (params (OverlappedComponent :type "PrimitiveComponent Object Reference") (OtherActor :type "Actor Object Reference") (OtherComp :type "PrimitiveComponent Object Reference") (OtherBodyIndex :type Integer))
  (bind _arrayoftarget (`self.ArrayOfTarget`))
  (`KismetArrayLibrary.Array_Remove` _arrayoftarget (`KismetArrayLibrary.Array_Find` _arrayoftarget OtherActor)))

(fn `AddInArray`
  (params (Object :type "Object Object Reference"))
  (bind _asbp_ennemy_01 (cast `/Game/Blueprints/Ennemy/BP_Ennemy01` Object)
    (:`then`
      (`KismetArrayLibrary.Array_Add` (`self.ArrayOfTarget`) _asbp_ennemy_01))
    (:`CastFailed`
      (bind _asbp_ennemy_02 (cast `/Game/Blueprints/Ennemy/BP_Ennemy02` Object)
        (:`then`
          (`KismetArrayLibrary.Array_Add` (`self.ArrayOfTarget`) _asbp_ennemy_02))
        (:`CastFailed`
          (bind _asbp_ennemy_03 (cast `/Game/Blueprints/Ennemy/BP_Ennemy03` Object))
          (`KismetArrayLibrary.Array_Add` (`self.ArrayOfTarget`) _asbp_ennemy_03))))))

(fn `Attack`
  (params (Index :type Integer))
  (returns (b_Continue :type Boolean))
  (bind _output (`self.ChooseTarget` Index))
  (bind _asbp_ennemy_01 (cast `/Game/Blueprints/Ennemy/BP_Ennemy01` _output)
    (:`then`
      (`/Game/Blueprints/Ennemy/BP_Ennemy01.TakeDamage` _asbp_ennemy_01 (`self.Damage`))
      (`ActorComponent.Activate` (`self.NS_SmokeBurst`) false)
      (return true))
    (:`CastFailed`
      (bind _asbp_ennemy_02 (cast `/Game/Blueprints/Ennemy/BP_Ennemy02` _output)
        (:`then`
          (`/Game/Blueprints/Ennemy/BP_Ennemy02.TakeDamage` _asbp_ennemy_02 (`self.Damage`))
          (`ActorComponent.Activate` (`self.NS_SmokeBurst`) false)
          (return true))
        (:`CastFailed`
          (bind _asbp_ennemy_03 (cast `/Game/Blueprints/Ennemy/BP_Ennemy03` _output)
            (:`then`
              (`/Game/Blueprints/Ennemy/BP_Ennemy03.TakeDamage` _asbp_ennemy_03 (`self.Damage`))
              (`ActorComponent.Activate` (`self.NS_SmokeBurst`) false)
              (return true))
            (:`CastFailed`
              (`KismetArrayLibrary.Array_Remove` (`self.ArrayOfTarget`))
              (return false))))))))

(fn `ChooseTarget`
  (params (Index :type Integer))
  (returns (Output :type "Actor Object Reference"))
  (return (`|GetArrayItem` (`self.ArrayOfTarget`) Index)))

(fn `LookTarget`
  (params (Target :type "Vector Structure (by ref)"))
  (`SceneComponent.K2_SetWorldRotation` (`self.StaticMesh`) (`KismetMathLibrary.FindLookAtRotation` (`SceneComponent.K2_GetComponentLocation` (`self.StaticMesh`)) Target) false false))

(fn `UserConstructionScript`)