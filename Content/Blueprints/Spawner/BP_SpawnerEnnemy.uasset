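; Enemy spawner that releases a wave of enemies at its mesh location and assigns each its spline.
; SpawnEnemie calls itself after a short random delay until the wave's remaining count runs out.
; IncreaseWave grows the enemy count randomly after wave one, then starts spawning.
; Enemy type is rolled by percentage, with variants 03 and 02 unlocking at later waves read from BP_SpanwerMaster.
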(event `self.ReceiveBeginPlay`
  (bind _returnvalue (`GameplayStatics.GetActorOfClass` "/Game/Blueprints/Spawner/BP_SpanwerMaster.BP_SpanwerMaster_C"))
  (set `self.MasterRef` _returnvalue))

(event `SpawnEnemie`
  (if (`self.CurrentWaveCheck`)
    (bind _returnvalue (`|SpawnActorFromClass` (`self.ChooseEnnemyToSpawn`) (`KismetMathLibrary.MakeTransform` (`SceneComponent.K2_GetComponentLocation` (`self.StaticMesh`))) "Undefined" "OverrideRootScale" null null))
    (`self.GiveSpline` _returnvalue)
    (`KismetSystemLibrary.Delay` (`KismetMathLibrary.RandomFloatInRange` 0.2 1.0))
    (set `self.enemy remaining` (- (`self.enemy remaining`) 1))
    (`self.SpawnEnemie`)))

(fn `ChooseEnnemyToSpawn`
  (returns (ClassToSpawn :type "Actor Class Reference"))
  (locals (PercentEnnemy03 :type "Float (double-precision)" :default 20.0) (PercentEnnemy02 :type "Float (double-precision)" :default 20.0))
  (if (<= (`/Game/Blueprints/Spawner/BP_SpanwerMaster.NumberOfCurrentWave` (`self.MasterRef`)) 1)
    (return "/Game/Blueprints/Ennemy/BP_Ennemy01.BP_Ennemy01_C")
    (elif (and (<= (`KismetMathLibrary.RandomFloatInRange` 0.0 100.0) (`local.PercentEnnemy02`)) (>= (`/Game/Blueprints/Spawner/BP_SpanwerMaster.NumberOfCurrentWave` (`self.MasterRef`)) 5))
      (return "/Game/Blueprints/Ennemy/BP_Ennemy02.BP_Ennemy02_C")
      (elif (and (<= (`KismetMathLibrary.RandomFloatInRange` 0.0 100.0) (`local.PercentEnnemy03`)) (>= (`/Game/Blueprints/Spawner/BP_SpanwerMaster.NumberOfCurrentWave` (`self.MasterRef`)) 3))
        (return "/Game/Blueprints/Ennemy/BP_Ennemy03.BP_Ennemy03_C")
        (else
          (return "/Game/Blueprints/Ennemy/BP_Ennemy01.BP_Ennemy01_C"))))))

(fn `CurrentWaveCheck`
  (returns (b_RemainingEnnemy :type Boolean))
  (return (not (<= (`self.enemy remaining`) 0))))

(fn `GiveSpline`
  (params (CurrentSpawn :type "Object Object Reference"))
  (bind _asbp_ennemy_01 (cast `/Game/Blueprints/Ennemy/BP_Ennemy01` CurrentSpawn)
    (:`then`
      (set `/Game/Blueprints/Ennemy/BP_Ennemy01.Spline` (`self.SplineRef`) _asbp_ennemy_01))
    (:`CastFailed`
      (bind _asbp_ennemy_02 (cast `/Game/Blueprints/Ennemy/BP_Ennemy02` CurrentSpawn)
        (:`then`
          (set `/Game/Blueprints/Ennemy/BP_Ennemy02.Spline` (`self.SplineRef`) _asbp_ennemy_02))
        (:`CastFailed`
          (bind _asbp_ennemy_03 (cast `/Game/Blueprints/Ennemy/BP_Ennemy03` CurrentSpawn))
          (set `/Game/Blueprints/Ennemy/BP_Ennemy03.Spline` (`self.SplineRef`) _asbp_ennemy_03))))))

(fn `Increase Wave`
  (if (not (== (`/Game/Blueprints/Spawner/BP_SpanwerMaster.NumberOfCurrentWave` (`self.MasterRef`)) 1))
    (bind _output_get (set `self.NumberOfEnnemys` (+ (`self.NumberOfEnnemys`) (`KismetMathLibrary.RandomIntegerInRange` 0 3))))
    (set `self.enemy remaining` _output_get))
  (`self.SpawnEnemie`))

(fn `UserConstructionScript`)