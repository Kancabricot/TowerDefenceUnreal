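; Wave manager actor that advances enemy waves across all BP_SpawnerEnnemy spawners in the level.
; It caches every spawner at BeginPlay, and its CheckEnnemyOnMap event waits briefly before testing whether any actor of the three enemy classes remains.
; Once none remain, it increments the wave counter and calls IncreaseWave on each spawner whose StartWave has been reached.
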(event `self.ReceiveBeginPlay`
  (bind _outactors (`GameplayStatics.GetAllActorsOfClass` "/Game/Blueprints/Spawner/BP_SpawnerEnnemy.BP_SpawnerEnnemy_C"))
  (set `self.SpanwerRef` _outactors))

(event `CheckEnnemyOnMap`
  (`KismetSystemLibrary.Delay` 0.2)
  (if (`self.CheckEnnemy`)
    (set `self.NumberOfCurrentWave` (+ (`self.NumberOfCurrentWave`) 1))
    (for _array_element (`self.SpanwerRef`)
      (if (<= (`/Game/Blueprints/Spawner/BP_SpawnerEnnemy.StartWave` _array_element) (`self.NumberOfCurrentWave`))
        (`/Game/Blueprints/Spawner/BP_SpawnerEnnemy.Increase Wave` _array_element)))))

(fn `CheckEnnemy`
  (returns (ReturnValue :type Boolean))
  (bind _outactors (`GameplayStatics.GetAllActorsOfClass` "/Game/Blueprints/Ennemy/BP_Ennemy01.BP_Ennemy01_C"))
  (bind _outactors_2 (`GameplayStatics.GetAllActorsOfClass` "/Game/Blueprints/Ennemy/BP_Ennemy02.BP_Ennemy02_C"))
  (bind _outactors_3 (`GameplayStatics.GetAllActorsOfClass` "/Game/Blueprints/Ennemy/BP_Ennemy03.BP_Ennemy03_C"))
  (return (and (<= (`KismetArrayLibrary.Array_Length` _outactors) 0) (<= (`KismetArrayLibrary.Array_Length` _outactors_2) 0) (<= (`KismetArrayLibrary.Array_Length` _outactors_3) 0))))

(fn `UserConstructionScript`)