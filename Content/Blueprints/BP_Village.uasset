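; BP_Village is the base the player defends, losing life when enemies reach its Trigger volume.
; On overlap it casts to three enemy classes, applies that enemy's DamageDo, destroys it and asks MasterRef to check the enemies left on the map.
; ApplyDamage subtracts from LifePoint and shows the WG_LooseMenu widget once CheckLife finds it at zero or below.
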(event `self.Trigger.OnComponentBeginOverlap`
  (params (OverlappedComponent :type "PrimitiveComponent Object Reference") (OtherActor :type "Actor Object Reference") (OtherComp :type "PrimitiveComponent Object Reference") (OtherBodyIndex :type Integer) (bFromSweep :type Boolean) (SweepResult :type "HitResult Structure (by ref)"))
  (bind _asbp_ennemy_01 (cast `/Game/Blueprints/BP_Ennemy01` OtherActor)
    (:`then`
      (`self.ApplyDamage` (`/Game/Blueprints/BP_Ennemy01.DamageDo` _asbp_ennemy_01)))
    (:`CastFailed`
      (bind _asbp_ennemy_02 (cast `/Game/Blueprints/BP_Ennemy02` OtherActor)
        (:`then`
          (`self.ApplyDamage` (`/Game/Blueprints/BP_Ennemy02.DamageDo` _asbp_ennemy_02)))
        (:`CastFailed`
          (bind _asbp_ennemy_03 (cast `/Game/Blueprints/BP_Ennemy03` OtherActor))
          (`self.ApplyDamage` (`/Game/Blueprints/BP_Ennemy03.DamageDo` _asbp_ennemy_03))))))
  (`self.K2_DestroyActor` _asbp_ennemy_01)
  (`/Game/Blueprints/BP_SpanwerMaster.CheckEnnemyOnMap` (`self.MasterRef`)))

(fn `ApplyDamage`
  (params (DamageTaken :type "Float (double-precision)"))
  (set `self.LifePoint` (- (`self.LifePoint`) DamageTaken))
  (if (`self.CheckLife`)
    (bind _returnvalue (`|CreateWidget` "/Game/UI/WG_LooseMenu.WG_LooseMenu_C"))
    (`UserWidget.AddToViewport` _returnvalue 0)))

(fn `CheckLife`
  (returns (IsAlive :type Boolean))
  (return (<= (`self.LifePoint`) 0.0)))

(fn `UserConstructionScript`)