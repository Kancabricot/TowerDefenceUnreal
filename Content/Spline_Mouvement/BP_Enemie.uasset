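; BP_Enemie is an enemy actor that travels along a referenced spline from start to end.
; After a short delay on BeginPlay, a Timeline plays at a rate of 1/Speed, so a higher Speed value means slower travel.
; Each update maps the Timeline alpha to spline distance, setting world location and tangent-aligned rotation.
; It also caches the BP_SpawnerEnnemy actors in Spawner, which is unused in this graph.
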(event `self.ReceiveBeginPlay`
  (bind _spline (`/Game/Spline_Mouvement/spline_mouvement.Spline` (`self.Spline`)))
  (`|ExecutionSequence`
    (:`then_0`
      (bind _outactors (`GameplayStatics.GetAllActorsOfClass` "/Game/ThirdPerson/Blueprints/BP_SpawnerEnnemy.BP_SpawnerEnnemy_C"))
      (set `self.Spawner` _outactors))
    (:`then_1`
      (`KismetSystemLibrary.Delay` 0.2)
      (`TimelineComponent.SetPlayRate` (`self.Timeline`) (/ 1.0 (`self.Speed`)))
      (bind (_direction _newtrack_0) (`Timeline|Timeline` :!via `PlayFromStart`)
        (:`Update`
          (bind _returnvalue (`KismetMathLibrary.Lerp` 0.0 (`SplineComponent.GetDistanceAlongSplineAtSplinePoint` _spline (- (`SplineComponent.GetNumberOfSplinePoints` _spline) 1)) _newtrack_0))
          (`self.K2_SetActorLocation` (`SplineComponent.GetLocationAtDistanceAlongSpline` _spline _returnvalue "World"))
          (`self.K2_SetActorRotation` (`KismetMathLibrary.Conv_VectorToRotator` (`SplineComponent.GetTangentAtDistanceAlongSpline` _spline _returnvalue "World"))))))))

(fn `UserConstructionScript`)